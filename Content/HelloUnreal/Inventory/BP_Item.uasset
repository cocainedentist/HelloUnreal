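; BP_Item is a world item pickup that passes itself to an overlapping actor's inventory by row name.
; The construction script looks up ItemRowName in DT_Item and sets the static mesh from that row.
; When the mesh begins overlapping an actor with an InventoryConponent, it calls AddItem with the row name.
; The item destroys itself when AddItem returns false.
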(event OnComponentBeginOverlap(StaticMesh)
  (params (OverlappedComponent :type Primitive%20Component%20Object%20Reference) (OtherActor :type Actor%20Object%20Reference) (OtherComp :type Primitive%20Component%20Object%20Reference) (OtherBodyIndex :type Integer) (bFromSweep :type Boolean) (SweepResult :type Hit%20Result%20Structure%20%28by%20ref%29))
  (bind _returnvalue (Actor|GetComponentbyClass OtherActor "/Game/HelloUnreal/Inventory/InventoryConponent.InventoryConponent_C"))
  (Utilities|IsValid _returnvalue
    (:Is%20Valid
      (bind _isfail (Default|AddItem _returnvalue (Variables|Default|GetItemRowName)))
      (if (not _isfail)
        (Actor|DestroyActor)))))

(fn ConstructionScript
  (bind _returnvalue (Utilities|GetDataTableRow "/Game/HelloUnreal/Inventory/DT_Item.DT_Item" (Variables|Default|GetItemRowName))
    (:then
      (Components|StaticMesh|SetStaticMesh (Variables|Default|GetStaticMesh) (.StaticMesh (Utilities|Struct|BreakST_Item _returnvalue))))))