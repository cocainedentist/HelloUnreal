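; BP_Switch is an interactable switch that turns play/stop on and off when a character triggers its press-F event.
; EventPressF calls TriggerSwitch, which flips the Toggle boolean and broadcasts it through an event dispatcher, so listeners react without direct references.
; EventPlay, EventReleaseF and the cube overlap are empty.
; An alternative loop calling BPI_PlayStop on an Actors array remains disconnected, alongside other unused array-node experiments.
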(event OnComponentBeginOverlap(myCube)
  (params (OverlappedComponent :type Primitive%20Component%20Object%20Reference) (OtherActor :type Actor%20Object%20Reference) (OtherComp :type Primitive%20Component%20Object%20Reference) (OtherBodyIndex :type Integer) (bFromSweep :type Boolean) (SweepResult :type Hit%20Result%20Structure%20%28by%20ref%29)))

(event Custom|TriggerSwitch
  (bind _output_get (Variables|Default|SetToggle (not (Variables|Default|GetToggle))))
  (Default|CallNewEventDispatcherPlayStop _output_get))

(fn ConstructionScript)

(fn EventPlay
  (params (isPlay :type Boolean))
  (return false))

(fn EventPressF
  (params (Character :type Character%20Object%20Reference))
  (CallFunction|TriggerSwitch)
  (return false))

(fn EventReleaseF
  (return false))