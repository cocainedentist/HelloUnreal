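; BP_Rect is an actor that moves its TripleA component around a square path in the local X-Z plane.
; Each Tick, a MoveType state selects one of four directional functions and switches to the next direction when the position passes that side's bound.
; Each function steps LocationX or LocationZ by a fixed amount and applies both as TripleA's relative location, so speed depends on frame rate.
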(event EventTick
  (params (DeltaSeconds :type Float%20%28single-precision%29))
  (switch Utilities|FlowControl|Switch|SwitchonEN_MoveType (Variables|Default|GetmoveType)
    (:NewEnumerator11
      (CallFunction|MoveRight)
      (if (>= (Variables|Default|GetlocationX) 5e+02)
        (Variables|Default|SetmoveType "NewEnumerator12")))
    (:NewEnumerator12
      (CallFunction|MoveUp)
      (if (>= (Variables|Default|GetlocationZ) 5e+02)
        (Variables|Default|SetmoveType "NewEnumerator13")))
    (:NewEnumerator13
      (CallFunction|MoveLeft)
      (if (< (Variables|Default|GetlocationX) 0.0)
        (Variables|Default|SetmoveType "NewEnumerator14")))
    (:NewEnumerator14
      (CallFunction|MoveDown)
      (if (< (Variables|Default|GetlocationZ) 0.0)
        (Variables|Default|SetmoveType "NewEnumerator11")))))

(fn ConstructionScript)

(fn MoveRight
  ;[0.15 0.15 0.15 0.5] Move Right
  (bind _output_get (Variables|Default|SetlocationX (+ (Variables|Default|GetlocationX) 2.0)))
  (Transformation|SetRelativeLocation (Variables|Default|GetTripleA) (Math|Vector|MakeVector _output_get 0.0 (Variables|Default|GetlocationZ)) false false))

(fn MoveUp
  ;[0.15 0.15 0.15 0.5] Move Up
  (bind _output_get (Variables|Default|SetlocationZ (+ (Variables|Default|GetlocationZ) 2.0)))
  (Transformation|SetRelativeLocation (Variables|Default|GetTripleA) (Math|Vector|MakeVector (Variables|Default|GetlocationX) 0.0 _output_get) false false))

(fn MoveLeft
  ;[0.15 0.15 0.15 0.5] Move Left
  (bind _output_get (Variables|Default|SetlocationX (- (Variables|Default|GetlocationX) 2.0)))
  (Transformation|SetRelativeLocation (Variables|Default|GetTripleA) (Math|Vector|MakeVector _output_get 0.0 (Variables|Default|GetlocationZ)) false false))

(fn MoveDown
  ;[0.15 0.15 0.15 0.5] Move Down
  (bind _output_get (Variables|Default|SetlocationZ (- (Variables|Default|GetlocationZ) 2.0)))
  (Transformation|SetRelativeLocation (Variables|Default|GetTripleA) (Math|Vector|MakeVector (Variables|Default|GetlocationX) 0.0 _output_get) false false))