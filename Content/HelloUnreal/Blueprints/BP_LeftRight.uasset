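; BP_LeftRight is an Actor that slides its TripleA component back and forth along relative X between fixed bounds.
; Tick checks IsMoveRight, calls MoveRight or MoveLeft to step LocationX by a fixed per-frame amount without delta-time scaling, and flips the flag at each bound.
; The Construction Script gives TripleA a dynamic instance of M_Mask_Inst and sets its Color parameter.
; BeginPlay prints a string on screen.
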(event EventTick
  (params (DeltaSeconds :type Float%20%28single-precision%29))
  (if (Variables|Default|GetisMoveRight)
    (CallFunction|MoveRight)
    (if (>= (Variables|Default|GetlocationX) 5e+02)
      (Variables|Default|SetisMoveRight false))
    (else
      (CallFunction|MoveLeft)
      (if (<= (Variables|Default|GetlocationX) 0.0)
        (Variables|Default|SetisMoveRight true)))))

(event EventBeginPlay
  ;[0.15 0.15 0.15 0.5] When this Actor plays
  ;[0.15 0.15 0.15 0.5] print string on screen
  (Development|PrintString "Hello"))

(fn ConstructionScript
  (bind _returnvalue (Rendering|Material|CreateDynamicMaterialInstance (Variables|Default|GetTripleA) 0 "/Game/HelloUnreal/StartUnreal/M_Mask_Inst.M_Mask_Inst" "None" :!class /Script/Engine.PrimitiveComponent))
  (Rendering|Material|SetVectorParameterValue _returnvalue "Color" (Variables|Default|GetValue) :!class /Script/Engine.MaterialInstanceDynamic))

(fn MoveRight
  ;[0.15 0.15 0.15 0.5] Move Right
  (bind _output_get (Variables|Default|SetlocationX (+ (Variables|Default|GetlocationX) 2.0)))
  (Transformation|SetRelativeLocation (Variables|Default|GetTripleA) (Math|Vector|MakeVector _output_get 0.0 0.0) false false))

(fn MoveLeft
  ;[0.15 0.15 0.15 0.5] Move Left
  (bind _output_get (Variables|Default|SetlocationX (- (Variables|Default|GetlocationX) 2.0)))
  (Transformation|SetRelativeLocation (Variables|Default|GetTripleA) (Math|Vector|MakeVector _output_get 0.0 0.0) false false))