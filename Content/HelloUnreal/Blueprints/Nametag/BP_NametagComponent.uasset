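; BP_NametagComponent is a component that gives its owning Character an on-screen nametag showing HP.
; On BeginPlay it creates the nametag widget, adds it to the viewport, then binds to the owner's StatComponent HP dispatcher and pushes the initial values.
; Each Tick it passes its world location to the widget, which it removes on EndPlay.
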(event EventBeginPlay
  (bind _returnvalue (Components|GetOwner))
  (bind _returnvalue_2 (Actor|GetComponentbyClass _returnvalue "/Game/HelloUnreal/AI/StatComponent.StatComponent_C"))
  (CallFunction|CreateWidget)
  (Utilities|IsValid _returnvalue_2
    (:Is%20Valid
      (EventDispatchers|BindEventtoEventDispatcherUpdateHP _returnvalue_2 (EventDispatchers|CreateEvent :!event UpdateHP))
      (CallFunction|UpdateHP (Variables|/Game/HelloUnreal/AI/StatComponent.StatComponent_C|GetCurrentHP _returnvalue_2) (Variables|/Game/HelloUnreal/AI/StatComponent.StatComponent_C|GetMaxHP _returnvalue_2)))
    (:Is%20Not%20Valid
      (Development|PrintString "No s c"))))

(event EventTick
  (params (DeltaSeconds :type Float%20%28single-precision%29))
  (bind _nametagwidget (Variables|Default|GetNametagWidget)
    (:then
      (Default|UpdateNametag _nametagwidget (Transformation|GetWorldLocation)))
    (:else)))

(event EventEndPlay
  (params (EndPlayReason :type EEndPlayReason%20Enum :default "Destroyed"))
  (bind _nametagwidget (Variables|Default|GetNametagWidget)
    (:then
      (Widget|RemovefromParent _nametagwidget))
    (:else)))

(fn UpdateHP
  (params (CurrentHP :type Float%20%28double-precision%29) (MaxHP :type Float%20%28double-precision%29))
  (Default|UpdateHP (Variables|Default|GetNametagWidget) CurrentHP MaxHP))

(fn CreateWidget
  (bind _ascharacter (Utilities|Casting|CastToCharacter (Components|GetOwner)))
  (bind _returnvalue (UserInterface|CreateWidget "/Game/HelloUnreal/Blueprints/Nametag/NametagWidget.NametagWidget_C" 0 _ascharacter))
  (bind _output_get (Variables|Default|SetNametagWidget _returnvalue))
  (UserInterface|Viewport|AddtoViewport _output_get 0))