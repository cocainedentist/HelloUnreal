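; BP_Dummy is a damageable dummy actor with a health display on its widget component.
; It starts at full HP, subtracts incoming AnyDamage, and passes current and max HP to HPWidget through PrintWidget, which also destroys the actor once HP reaches zero.
; Every tick, UpdateLookCamera turns the widget toward the player camera using only X and Y positions, so it rotates horizontally without tilting.
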(event Game|Damage|EventAnyDamage
  (params (Damage :type Float%20%28single-precision%29) (DamageType :type Damage%20Type%20Object%20Reference) (InstigatedBy :type Controller%20Object%20Reference) (DamageCauser :type Actor%20Object%20Reference))
  (Variables|Default|SetCurrentHP (- (Variables|Default|GetCurrentHP) Damage))
  (CallFunction|PrintWidget))

(event EventBeginPlay
  (Variables|Default|SetCurrentHP 1e+02)
  (Variables|Default|SetMaxHP 1e+02)
  (CallFunction|PrintWidget))

(event EventTick
  (params (DeltaSeconds :type Float%20%28single-precision%29))
  (CallFunction|UpdateLookCamera))

(fn ConstructionScript)

(fn PrintWidget
  (Utilities|FlowControl|Sequence
    (:then_0
      (bind _asdummy_hpwidget (Utilities|Casting|CastToHPWidget (UserInterface|GetUserWidgetObject (Variables|Default|GetWidget))))
      (Default|SetHP _asdummy_hpwidget (Variables|Default|GetCurrentHP) (Variables|Default|GetMaxHP))
      (if (<= (Variables|Default|GetCurrentHP) 0.0)
        (Actor|DestroyActor)))))

(fn UpdateLookCamera
  (bind _returnvalue (Game|GetPlayerCameraManager 0))
  (bind _widget (Variables|Default|GetWidget))
  (bind _returnvalue_2 (Transformation|GetActorLocation _returnvalue))
  (bind _returnvalue_3 (Transformation|GetWorldLocation _widget))
  (Transformation|SetWorldRotation (Variables|Default|GetWidget) (Math|Rotator|FindLookatRotation (Math|Vector|MakeVector (.x _returnvalue_3) (.y _returnvalue_3) 0.0) (Math|Vector|MakeVector (.x _returnvalue_2) (.y _returnvalue_2) 0.0)) false false))