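; BP_Rect1 is an actor that moves its TripleA component along a repeating path in the relative X-Z plane.
; Each Tick switches on MoveType, steps LocationX or LocationZ by a fixed per-frame amount with no delta-time scaling, and applies it as relative location.
; Threshold checks chain Right, Up, Down, Left, so despite the Rect name the component retraces an L shape instead of a rectangle.
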(event EventTick
  (params (DeltaSeconds :type Float%20%28single-precision%29))
  (switch Utilities|FlowControl|Switch|SwitchonEN_MoveType (Variables|Default|GetmoveType)
    (:NewEnumerator11
      ;[0.15 0.15 0.15 0.5] Move Right
      (bind _output_get (Variables|Default|SetlocationX (+ (Variables|Default|GetlocationX) 2.0)))
      (Transformation|SetRelativeLocation (Variables|Default|GetTripleA) (Math|Vector|MakeVector _output_get 0.0 (Variables|Default|GetlocationZ)) false false)
      (if (>= (Variables|Default|GetlocationX) 5e+02)
        (Variables|Default|SetmoveType "NewEnumerator12")))
    (:NewEnumerator12
      ;[0.15 0.15 0.15 0.5] Move Up
      (bind _output_get_2 (Variables|Default|SetlocationZ (+ (Variables|Default|GetlocationZ) 2.0)))
      (Transformation|SetRelativeLocation (Variables|Default|GetTripleA) (Math|Vector|MakeVector (Variables|Default|GetlocationX) 0.0 _output_get_2) false false)
      (if (>= (Variables|Default|GetlocationZ) 5e+02)
        (Variables|Default|SetmoveType "NewEnumerator14")))
    (:NewEnumerator13
      ;[0.15 0.15 0.15 0.5] Move Left
      (bind _output_get_3 (Variables|Default|SetlocationX (- (Variables|Default|GetlocationX) 2.0)))
      (Transformation|SetRelativeLocation (Variables|Default|GetTripleA) (Math|Vector|MakeVector _output_get_3 0.0 (Variables|Default|GetlocationZ)) false false)
      (if (< (Variables|Default|GetlocationX) 0.0)
        (Variables|Default|SetmoveType "NewEnumerator11")))
    (:NewEnumerator14
      ;[0.15 0.15 0.15 0.5] Move Down
      (bind _output_get_4 (Variables|Default|SetlocationZ (- (Variables|Default|GetlocationZ) 2.0)))
      (Transformation|SetRelativeLocation (Variables|Default|GetTripleA) (Math|Vector|MakeVector (Variables|Default|GetlocationX) 0.0 _output_get_4) false false)
      (if (< (Variables|Default|GetlocationZ) 0.0)
        (Variables|Default|SetmoveType "NewEnumerator13")))))

(fn ConstructionScript)