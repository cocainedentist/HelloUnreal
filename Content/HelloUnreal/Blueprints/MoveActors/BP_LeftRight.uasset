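; BP_LeftRight is an actor that slides its TripleA component back and forth along the X axis while play is enabled.
; Each Tick steps a stored LocationX by a fixed, frame-rate-dependent amount through MoveRight or MoveLeft, then applies it as relative location.
; A direction flag flips when the position reaches either end of its range.
; EventPlay sets the IsPlay flag that gates the motion.
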(event EventTick
  (params (DeltaSeconds :type Float%20%28single-precision%29))
  (if (Variables|Default|GetisPlay)
    (if (Variables|Default|GetisMoveRight)
      (CallFunction|MoveRight)
      (if (>= (Variables|Default|GetlocationX) 5e+02)
        (Variables|Default|SetisMoveRight false))
      (else
        (CallFunction|MoveLeft)
        (if (<= (Variables|Default|GetlocationX) 0.0)
          (Variables|Default|SetisMoveRight true))))))

(fn ConstructionScript)

(fn MoveRight
  ;[0.15 0.15 0.15 0.5] Move Right
  (bind _output_get (Variables|Default|SetlocationX (+ (Variables|Default|GetlocationX) 2.0)))
  (Transformation|SetRelativeLocation (Variables|Default|GetTripleA) (Math|Vector|MakeVector _output_get 0.0 0.0) false false))

(fn MoveLeft
  ;[0.15 0.15 0.15 0.5] Move Left
  (bind _output_get (Variables|Default|SetlocationX (- (Variables|Default|GetlocationX) 2.0)))
  (Transformation|SetRelativeLocation (Variables|Default|GetTripleA) (Math|Vector|MakeVector _output_get 0.0 0.0) false false))

(fn EventPlay
  (params (isPlay :type Boolean))
  (bind _output_get (Variables|Default|SetisPlay isPlay))
  (return _output_get))