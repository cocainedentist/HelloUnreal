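; BP_SplineMove is an actor that moves a cube along its spline in a repeating loop.
; A timeline scales its value by spline length, and each update sets the cube's world location and rotation from the spline transform at that distance.
; On finish the timeline replays from the start, while EventPlay takes a boolean to trigger the play or stop events.
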(event Custom|doPlay
  (bind _value (Timeline|Timeline Play)
    (:Update
      (Transformation|SetWorldLocationAndRotation (Variables|Default|GetCube) (.location (Spline|GetTransformatDistanceAlongSpline (Variables|Default|GetSpline) (* (Spline|GetSplineLength (Variables|Default|GetSpline)) _value) "World" false)) (.rotation (Spline|GetTransformatDistanceAlongSpline (Variables|Default|GetSpline) (* (Spline|GetSplineLength (Variables|Default|GetSpline)) _value) "World" false)) false false))
    (:Finished
      (Timeline|Timeline PlayFromStart))))

(event Custom|doStop
  (bind _value (Timeline|Timeline Stop)
    (:Update
      (Transformation|SetWorldLocationAndRotation (Variables|Default|GetCube) (.location (Spline|GetTransformatDistanceAlongSpline (Variables|Default|GetSpline) (* (Spline|GetSplineLength (Variables|Default|GetSpline)) _value) "World" false)) (.rotation (Spline|GetTransformatDistanceAlongSpline (Variables|Default|GetSpline) (* (Spline|GetSplineLength (Variables|Default|GetSpline)) _value) "World" false)) false false))
    (:Finished
      (Timeline|Timeline PlayFromStart))))

(fn ConstructionScript)

(fn EventPlay
  (params (isPlay :type Boolean))
  (if isPlay
    (CallFunction|DoPlay)
    (else
      (CallFunction|DoStop)))
  (return false))