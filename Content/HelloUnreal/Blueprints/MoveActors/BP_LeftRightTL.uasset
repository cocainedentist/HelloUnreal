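; BP_LeftRightTL is an actor that slides a cube back and forth, left and right as its name suggests, using a Timeline.
; Each update sets the Cube's relative location to the Scene component's relative location scaled by the timeline value, so that component defines the travel endpoint.
; On finish, IsMoveRight flips and selects Play or Reverse, creating a ping-pong loop.
; EventPlay starts or stops the motion through doPlay and doStop.
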(event Custom|doPlay
  (if (Variables|Default|GetisMoveRight) :!label _label
    (bind _value (Timeline|Timeline Play)
      (:Update
        (Transformation|SetRelativeLocation (Variables|Default|GetCube) (* _value (Variables|/Script/Engine.SceneComponent|GetRelativeLocation (Variables|Default|GetScene))) false false))
      (:Finished
        ;[0.15 0.15 0.15 0.5] Toggle
        (Variables|Default|SetisMoveRight (not (Variables|Default|GetisMoveRight)))
        (goto _label)))
    (else
      (Timeline|Timeline Reverse))))

(event Custom|doStop
  (bind _value (Timeline|Timeline Stop)
    (:Update
      (Transformation|SetRelativeLocation (Variables|Default|GetCube) (* _value (Variables|/Script/Engine.SceneComponent|GetRelativeLocation (Variables|Default|GetScene))) false false))
    (:Finished
      ;[0.15 0.15 0.15 0.5] Toggle
      (Variables|Default|SetisMoveRight (not (Variables|Default|GetisMoveRight)))
      (if (Variables|Default|GetisMoveRight)
        (Timeline|Timeline Play)
        (else
          (Timeline|Timeline Reverse))))))

(fn ConstructionScript)

(fn EventPlay
  (params (isPlay :type Boolean))
  (if isPlay
    (CallFunction|DoPlay)
    (else
      (CallFunction|DoStop)))
  (return false))