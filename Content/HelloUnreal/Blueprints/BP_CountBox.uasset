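; BP_CountBox is a counter box actor that shows how many times something has overlapped its cube.
; BeginPlay resets the count to zero and writes it to a TextRender component.
; Each Cube begin-overlap calls RenderCount, which increments the count, wraps it back to zero after nine, and updates the displayed text.
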(event OnComponentBeginOverlap(Cube)
  (params (OverlappedComponent :type Primitive%20Component%20Object%20Reference) (OtherActor :type Actor%20Object%20Reference) (OtherComp :type Primitive%20Component%20Object%20Reference) (OtherBodyIndex :type Integer) (bFromSweep :type Boolean) (SweepResult :type Hit%20Result%20Structure%20%28by%20ref%29))
  (CallFunction|RenderCount))

(event EventBeginPlay
  (bind _output_get (Variables|Default|Setcount 0))
  (Rendering|Components|TextRender|SetText (Variables|Default|GetTextRender) (Utilities|Text|ToText(Integer) _output_get)))

(fn ConstructionScript)

(fn RenderCount
  (bind _output_get (Variables|Default|Setcount (+ (Variables|Default|Getcount) 1)))
  (if (> (Variables|Default|Getcount) 9)
    (Variables|Default|Setcount 0)
    (Rendering|Components|TextRender|SetText (Variables|Default|GetTextRender) (Utilities|Text|ToText(Integer) _output_get))
    (else
      (Rendering|Components|TextRender|SetText (Variables|Default|GetTextRender) (Utilities|Text|ToText(Integer) _output_get)))))