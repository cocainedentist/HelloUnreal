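; Behavior Tree task that checks whether the controlled pawn is within attack range of the target actor held in a blackboard key.
; On AI execute it compares the distance between the two actor locations to a fixed threshold and, when closer, writes an EN_AIState value to the AI state key.
; Both branches finish the task as failed, so the blackboard write is its only differing result.
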(event EventReceiveExecuteAI
  (params (OwnerController :type AI%20Controller%20Object%20Reference) (ControlledPawn :type Pawn%20Object%20Reference))
  (if (< (Math|Vector|Distance(Vector) (Transformation|GetActorLocation ControlledPawn) (Transformation|GetActorLocation (AI|BehaviorTree|GetBlackboardValueasActor (Variables|Default|GetTargetKey)))) 1e+02)
    (Class|BTFunctionLibrary|SetBlackboardValueasEnum (Variables|Default|GetAIStateKey) (Utilities|Enum|LiteralenumEN_AIState "NewEnumerator2"))
    (AI|BehaviorTree|FinishExecute false)
    (else
      (AI|BehaviorTree|FinishExecute false))))