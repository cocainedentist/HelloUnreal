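; BP_Weapon is a weapon actor configured from a DT_Weapon row, which supplies its static mesh and attach socket.
; Construction applies the named row, and BeginPlay picks a random one when no name is set.
; It snaps onto a character's mesh socket, and detaching enables physics and clears the character.
; On hit notify, a sphere trace at the Hit socket applies fixed damage, while press/release F handlers are stubs.
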(event EventBeginPlay
  (if (== (Variables|Default|GetWeaponRowName) "None")
    (bind _outrownames (DataTable|GetDataTableRowNames "/Game/HelloUnreal/Data/DT_Weapon.DT_Weapon"))
    (bind _returnvalue (Utilities|GetDataTableRow "/Game/HelloUnreal/Data/DT_Weapon.DT_Weapon" (.OutItem (Utilities|Array|Random _outrownames)))
      (:then
        (bind _output_get (Variables|Default|SetWeaponData _returnvalue))
        (Components|StaticMesh|SetStaticMesh (Variables|Default|Getweapon) (.StaticMesh (Utilities|Struct|BreakST_Weapon _output_get)))))))

(fn ConstructionScript
  (bind _returnvalue (Utilities|GetDataTableRow "/Game/HelloUnreal/Data/DT_Weapon.DT_Weapon" (Variables|Default|GetWeaponRowName))
    (:then
      (bind _output_get (Variables|Default|SetWeaponData _returnvalue))
      (Components|StaticMesh|SetStaticMesh (Variables|Default|Getweapon) (.StaticMesh (Utilities|Struct|BreakST_Weapon _output_get))))))

(fn EventReleaseF
  (return false))

(fn EventPressF
  (params (Character :type Character%20Object%20Reference))
  (return false))

(fn AttachtoCharacter
  (params (Character :type Character%20Object%20Reference))
  (bind _output_get (Variables|Default|SetCharacter Character))
  (Transformation|AttachComponentToComponent (Variables|/Script/Engine.Character|GetMesh _output_get) (.socket (Variables|Default|GetWeaponData)) "SnapToTarget" "SnapToTarget" "KeepWorld" true)
  (return false))

(fn DetachtoCharacter
  (params (Character :type Character%20Object%20Reference))
  (Transformation|DetachFromActor "KeepWorld" "KeepWorld" "KeepWorld")
  (Physics|SetSimulatePhysics (Variables|Default|Getweapon) true)
  ;[0.15 0.15 0.15 0.5] 포인트를 비워뒀으니 null 처리다
  (Variables|Default|SetCharacter 0)
  (return false))

(fn EventNotifyHit
  (bind _weapon (Variables|Default|Getweapon))
  (bind _returnvalue (Transformation|GetSocketLocation _weapon "Hit"))
  (bind _outhit (Collision|SphereTraceForObjects _returnvalue _returnvalue 5e+01 (Utilities|Array|MakeArray "ObjectTypeQuery2") false 0 "ForDuration"))
  (Game|Damage|ApplyDamage (.HitActor (Collision|BreakHitResult _outhit)) 2e+01 (Pawn|GetController (Variables|Default|GetCharacter)) self)
  (return false))