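; BP_Cannon is an interactable cannon that fires one BP_CannonBall each time its press-F event is triggered.
; EventPressF calls ToggleCannon, which runs ShootCannon to spawn the ball at the Arrow component's location and rotation.
; Despite the toggle name, the looping-timer on/off logic with ON/OFF text is disconnected and never runs.
; The release-F and mesh overlap handlers are empty.
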(event OnComponentBeginOverlap(StaticMesh)
  (params (OverlappedComponent :type Primitive%20Component%20Object%20Reference) (OtherActor :type Actor%20Object%20Reference) (OtherComp :type Primitive%20Component%20Object%20Reference) (OtherBodyIndex :type Integer) (bFromSweep :type Boolean) (SweepResult :type Hit%20Result%20Structure%20%28by%20ref%29)))

(event Custom|ToggleCannon
  (CallFunction|ShootCannon))

(fn ConstructionScript)

(fn ShootCannon
  (bind _arrow (Variables|Default|GetArrow))
  (bind _returnvalue (Transformation|GetWorldTransform _arrow))
  (Game|SpawnActorfromClass "/Game/HelloUnreal/Blueprints/Cannon/BP_CannonBall.BP_CannonBall_C" (Math|Transform|MakeTransform (.location _returnvalue) (.rotation _returnvalue) "1.000000,1.000000,1.000000") "Undefined" "MultiplyWithRoot" 0 0))

(fn EventPressF
  (params (Character :type Character%20Object%20Reference))
  (CallFunction|ToggleCannon)
  (return false))

(fn EventReleaseF)